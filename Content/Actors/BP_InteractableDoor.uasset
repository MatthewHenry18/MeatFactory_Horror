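; Interactable door actor that the player opens with the InteractionStart input while overlapping it.
; Player overlap adds an InteractionPrompt widget and enables input on the actor if the door is still closed; end overlap disables input but leaves the widget untouched.
; Pressing the input calls OpenDoor, whose body is not in this graph, plays a sound at the door and sets DoorOpened.
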(event EventBeginPlay)

(event Collision|EventActorEndOverlap
  (params (OtherActor :type Actor%20Object%20Reference))
  (if (== (Game|GetPlayerCharacter 0) OtherActor)
    (Input|DisableInput (Game|GetPlayerController 0))))

(event EventTick
  (params (DeltaSeconds :type Float%20%28single-precision%29)))

(event Collision|EventActorBeginOverlap
  (params (OtherActor :type Actor%20Object%20Reference))
  ;[1 1 1] Opens the door on interaction pressed + Creates Interactive Prompt Widget
  (if (== (Game|GetPlayerCharacter 0) OtherActor)
    (if (not (Variables|Default|GetDoorOpened))
      (bind _returnvalue (UserInterface|CreateWidget "/Game/Widgets/InteractionPrompt.InteractionPrompt_C"))
      (UserInterface|Viewport|AddtoViewport _returnvalue 0)
      (Input|EnableInput (Game|GetPlayerController 0)))))

(event Input|ActionEvents|InputActionInteractionStart
  (params (Key :type Key%20Structure :default "None"))
  ;[1 1 1] Opens the door on interaction pressed + Creates Interactive Prompt Widget
  (:Pressed
    (Class|InteractableDoor|OpenDoor)
    (Audio|PlaySoundatLocation "/Engine/VREditor/Sounds/UI/Dockable_Window_Open.Dockable_Window_Open" (Transformation|GetActorLocation) "0, 0, 0" 4.0 1.0 0.0 0 0 0)
    (Variables|Default|SetDoorOpened true)))

(fn ConstructionScript)