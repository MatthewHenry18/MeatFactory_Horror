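; BP_CollectableKey is a key pickup actor that the player collects by pressing an interact input.
; When the player character overlaps its sphere collision, it shows an InteractionPrompt widget and enables input on itself.
; InteractionStart then calls HandleItemCollected on the overlapped AbstractionPlayerCharacter, plays a randomly pitched pickup sound and destroys the key.
; No end-overlap logic removes the prompt or disables input.
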(event OnComponentBeginOverlap(Cube)
  (params (OverlappedComponent :type Primitive%20Component%20Object%20Reference) (OtherActor :type Actor%20Object%20Reference) (OtherComp :type Primitive%20Component%20Object%20Reference) (OtherBodyIndex :type Integer) (bFromSweep :type Boolean) (SweepResult :type Hit%20Result%20Structure%20%28by%20ref%29)))

(event OnComponentBeginOverlap(SphereCollision)
  (params (OverlappedComponent :type Primitive%20Component%20Object%20Reference) (OtherActor :type Actor%20Object%20Reference) (OtherComp :type Primitive%20Component%20Object%20Reference) (OtherBodyIndex :type Integer) (bFromSweep :type Boolean) (SweepResult :type Hit%20Result%20Structure%20%28by%20ref%29))
  ;[1 1 1] Display widget
  (if (== (Game|GetPlayerCharacter 0) OtherActor)
    (bind _returnvalue (UserInterface|CreateWidget "/Game/Widgets/InteractionPrompt.InteractionPrompt_C"))
    (UserInterface|Viewport|AddtoViewport _returnvalue 0)
    (Input|EnableInput (Game|GetPlayerController 0))))

(event EventBeginPlay)

(event EventTick
  (params (DeltaSeconds :type Float%20%28single-precision%29)))

(event Input|ActionEvents|InputActionInteractionStart
  (params (Key :type Key%20Structure :default "None"))
  (:Pressed
    (bind _asabstraction_player_character (Utilities|Casting|CastToAbstractionPlayerCharacter (stale OnComponentBeginOverlap(SphereCollision) OtherActor)))
    (Class|AbstractionPlayerCharacter|HandleItemCollected _asabstraction_player_character)
    (Audio|PlaySoundatLocation "/Engine/VREditor/Sounds/UI/Object_PickUp.Object_PickUp" (Transformation|GetActorLocation) "0, 0, 0" 4.0 (Math|Random|RandomFloatinRange 0.8 1.2) 0.0 0 0 0)
    (Actor|DestroyActor)))

(fn ConstructionScript)