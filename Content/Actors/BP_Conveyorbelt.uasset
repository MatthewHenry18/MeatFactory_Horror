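; Conveyor belt actor that carries overlapping actors along its forward vector.
; Begin and end overlap events on a trigger box add actors to and remove them from a move list.
; Each Tick offsets every listed actor by the forward vector times BeltSpeed with sweep enabled.
; The offset is not scaled by delta time, so belt speed varies with frame rate.
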(event OnComponentBeginOverlap(ConveyorbeltTiggerBox)
  (params (OverlappedComponent :type Primitive%20Component%20Object%20Reference) (OtherActor :type Actor%20Object%20Reference) (OtherComp :type Primitive%20Component%20Object%20Reference) (OtherBodyIndex :type Integer) (bFromSweep :type Boolean) (SweepResult :type Hit%20Result%20Structure%20%28by%20ref%29))
  ;[1 1 1] Adds/Removes From Belt
  (Utilities|Array|AddUnique (Variables|Default|GetMoveList) OtherActor))

(event OnComponentEndOverlap(ConveyorbeltTiggerBox)
  (params (OverlappedComponent :type Primitive%20Component%20Object%20Reference) (OtherActor :type Actor%20Object%20Reference) (OtherComp :type Primitive%20Component%20Object%20Reference) (OtherBodyIndex :type Integer))
  ;[1 1 1] Adds/Removes From Belt
  (Utilities|Array|RemoveItem (Variables|Default|GetMoveList) OtherActor))

(event EventBeginPlay)

(event EventTick
  (params (DeltaSeconds :type Float%20%28single-precision%29))
  (for _array_element (Variables|Default|GetMoveList)
    (Transformation|AddActorWorldOffset _array_element (* (Transformation|GetActorForwardVector) (Variables|Default|GetBeltSpeed)) true)))

(fn ConstructionScript)